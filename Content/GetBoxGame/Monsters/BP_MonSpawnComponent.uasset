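; Monster spawner component that makes roughly one spawn attempt per second while its counter stays below 11.
; Each attempt picks a random point on a circle around the owner, sized by Radius times pi.
; A line trace from that point to a fixed world position below the origin must hit world geometry.
; It then spawns a random DT_Monster row's class as AI and passes the row name to SetMonstat.
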(event `self.ReceiveTick`
  (params (DeltaSeconds :type "Float (single-precision)"))
  (bind _output_get (set `self.TotalDeltaSeconds` (+ DeltaSeconds (`self.TotalDeltaSeconds`))))
  (if (== (`KismetMathLibrary.FFloor` _output_get) (`self.Count`))
    (if (< (`self.Count`) 11)
      (`self.DoSpawn`)
      (bind _output_get_2 (set `self.Count` (+ (`self.Count`) 1)))
      (`KismetSystemLibrary.PrintString` (`KismetStringLibrary.Concat_StrStr` "Monster Number : " (`KismetStringLibrary.Conv_IntToString` (- _output_get_2 1)))))))

(fn `DoSpawn`
  (locals (RandLocation :type "Vector Structure" :default (0.0 0.0 0.0)) (RowName :type Name))
  (bind _output_get (set `local.RandLocation` (`self.GetCircleLocation`)))
  (if (`self.IsCanSpawn` _output_get)
    (bind _outrownames (`DataTableFunctionLibrary.GetDataTableRowNames` "/Game/GetBoxGame/Monsters/DT_Monster.DT_Monster"))
    (bind _output_get_2 (set `local.RowName` (`KismetArrayLibrary.Array_Random` _outrownames)))
    (bind _returnvalue (`|GetDataTableRow` "/Game/GetBoxGame/Monsters/DT_Monster.DT_Monster" _output_get_2)
      (:`then`
        (bind _returnvalue_2 (`AIBlueprintHelperLibrary.SpawnAIFromClass` (`.MonsterClass_8_911F91BC4382E5CA3419E5AB88433DF3` (break `/Game/GetBoxGame/Monsters/ST_Monster` _returnvalue)) null (`local.RandLocation`) (struct) false null))
        (bind _asbp_monster_base (cast `/Game/GetBoxGame/Monsters/BP_MonsterBase` _returnvalue_2))
        (`/Game/GetBoxGame/Monsters/BP_MonsterBase.SetMonstat` _asbp_monster_base _output_get_2)))))

(fn `GetCircleLocation`
  (returns (ReturnValue :type "Vector Structure"))
  (locals (Rand :type "Float (double-precision)"))
  (bind _returnvalue (* (`self.Radius`) 3.141592))
  (bind _output_get (set `local.Rand` (`KismetMathLibrary.RandomFloatInRange` 0.0 360.0)))
  (return (+ (`Actor.K2_GetActorLocation` (`self.GetOwner`)) (`KismetMathLibrary.MakeVector` (* (`KismetMathLibrary.Cos` _output_get) _returnvalue) (* (`KismetMathLibrary.Sin` _output_get) _returnvalue)))))

(fn `IsCanSpawn`
  (params (WorldLocation :type "Vector Structure"))
  (returns (IsCanSpawn :type Boolean))
  (bind (_outhit _returnvalue) (`KismetSystemLibrary.LineTraceSingleForObjects` WorldLocation (+ (0.0 0.0 0.0) (0.0 0.0 -100.0)) (`|MakeArray` "ObjectTypeQuery1" "ObjectTypeQuery2" :!type "EObjectTypeQuery Enum")))
  (return _returnvalue))